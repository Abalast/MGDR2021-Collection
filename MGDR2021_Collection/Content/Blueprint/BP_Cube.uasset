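; BP_Cube is a small Blueprint with a health value and a Use input handler.
; BeginPlay sets Health to MaxHealth, and pressing Use only prints "Use".
; An unconnected chain would print Health in red and subtract Number from it, but it never runs; Tick and the construction script are empty.
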(event `self.ReceiveBeginPlay`
  ;[1 1 1] BeginPlay
  (set `self.Health` (`self.MaxHealth`)))

(event `self.ReceiveTick`
  (params (DeltaSeconds :type "Float (single-precision)"))
  ;[1 1 1] Tick Event
)

(event `InputAction|Use`
  (params (Key :type "Key Structure"))
  (:`Pressed`
    (`KismetSystemLibrary.PrintString` "Use")))

(event `InputAction|Jump`
  (params (Key :type "Key Structure")))

(fn `UserConstructionScript`)