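; BP_Item is a collectible pickup for the Roll The Ball game that adds one point to the player's score.
; Tick raises the actor's pitch by one degree each frame, independent of delta time, and prints the value.
; When the Cube component overlaps a BP_BallPlayer, it increments that player's Score, prints it in red and destroys itself.
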(event `self.ReceiveTick`
  (params (DeltaSeconds :type "Float (single-precision)"))
  (bind (_returnvalue_roll _returnvalue_pitch) (`KismetMathLibrary.BreakRotator` (`self.K2_GetActorRotation`)))
  (bind _returnvalue (+ _returnvalue_pitch 1.0))
  (`KismetSystemLibrary.PrintString` (`KismetStringLibrary.Conv_DoubleToString` _returnvalue))
  (`self.K2_SetActorRotation` (`KismetMathLibrary.MakeRotator` 0.0 _returnvalue)))

(event `self.Cube.OnComponentBeginOverlap`
  (params (OverlappedComponent :type "PrimitiveComponent Object Reference") (OtherActor :type "Actor Object Reference") (OtherComp :type "PrimitiveComponent Object Reference") (OtherBodyIndex :type Integer) (bFromSweep :type Boolean) (SweepResult :type "HitResult Structure (by ref)"))
  (bind _asbp_ball_player (cast `/Game/RollTheBall/Blueprint/PlayerCharacter/BP_BallPlayer` OtherActor))
  (bind _output_get (set `/Game/RollTheBall/Blueprint/PlayerCharacter/BP_BallPlayer.score` (+ (`/Game/RollTheBall/Blueprint/PlayerCharacter/BP_BallPlayer.score` _asbp_ball_player) 1) _asbp_ball_player))
  (`KismetSystemLibrary.PrintString` (`KismetStringLibrary.Conv_IntToString` _output_get) true true (struct :`R` 1.0 :`A` 1.0))
  (`self.K2_DestroyActor`))

(fn `UserConstructionScript`)