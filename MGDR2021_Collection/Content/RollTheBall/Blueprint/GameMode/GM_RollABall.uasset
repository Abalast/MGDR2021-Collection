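; GM_RollABall is the game mode for a roll-the-ball game, tracking score and a time limit.
; On BeginPlay it counts all BP_Item actors in the level to set HighScore.
; Tick accumulates elapsed time and prints it on screen, switching to a red "Game Over" message once MaxTime is reached.
; SetTheScore adds the passed amount to the running Score.
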(event `self.ReceiveBeginPlay`
  (bind _outactors (`GameplayStatics.GetAllActorsOfClass` "/Game/RollTheBall/Blueprint/Actor/BP_Item.BP_Item_C"))
  (bind _output_get (set `self.Out Actors` _outactors))
  (set `self.HighScore` (`KismetArrayLibrary.Array_Length` _output_get)))

(event `self.ReceiveTick`
  (params (DeltaSeconds :type "Float (single-precision)"))
  (bind _output_get (set `self.time` (+ (`self.time`) DeltaSeconds)))
  (if (>= (`self.time`) (`self.maxTime`))
    (`KismetSystemLibrary.PrintString` "Game Over" true true (struct :`R` 1.0 :`B` 0.016253 :`A` 1.0))
    (else
      (`KismetSystemLibrary.PrintString` (`KismetStringLibrary.Conv_DoubleToString` _output_get)))))

(fn `SetTheScore`
  (params (newScore :type Integer))
  (set `self.Score` (+ (`self.Score`) newScore)))

(fn `UserConstructionScript`)